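; BP_SliceableActor is an actor whose mesh can be cut along a plane at runtime.
; The construction script copies a chosen static mesh into a procedural mesh with collision, then destroys the source component.
; OnSlice cuts the overlapped procedural mesh at the impact point and normal, capping it with a slice material.
; The new half gets physics, a velocity impulse along the normal, and an overlap binding.
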(event EventBeginPlay)

(event Collision|EventActorBeginOverlap
  (params (OtherActor :type Actor%20Object%20Reference)))

(event EventTick
  (params (DeltaSeconds :type Float%20%28single-precision%29)))

(event EventOnSlice
  (params (ImpactPoint :type Vector%20%28by%20ref%29 :default "0, 0, 0") (Normal :type Vector%20%28by%20ref%29 :default "0, 0, 0") (CompOverlapped :type Procedural%20Mesh%20Component%20Object%20Reference))
  (bind _outotherhalfprocmesh (Class|KismetProceduralMeshLibrary|SliceProceduralMesh CompOverlapped ImpactPoint Normal true "CreateNewSectionForCap" (Variables|Default|Getm_capSliceMaterial)))
  (Physics|SetSimulatePhysics _outotherhalfprocmesh true)
  (Physics|AddImpulse _outotherhalfprocmesh (* Normal 1e+03) "None" true)
  (Class|SliceableActor|BindNewtoComptoBeginOverlap _outotherhalfprocmesh))

(fn ConstructionScript
  (Components|StaticMesh|SetStaticMesh (Variables|Default|Getm_baseMeshComp) (Variables|Default|Getm_meshToCopy))
  (Class|KismetProceduralMeshLibrary|CopyProceduralMeshfromStaticMeshComponent (Variables|Default|Getm_baseMeshComp) 0 (Variables|Default|Getm_meshProceduralComp) true)
  (Components|DestroyComponent (Variables|Default|Getm_baseMeshComp)))